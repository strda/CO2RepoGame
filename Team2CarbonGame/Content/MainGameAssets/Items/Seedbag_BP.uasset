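; Seedbag pickup actor that gets sucked toward a target and grants items to the robot character.
; While flagged as being sucked, Tick moves it at constant speed toward a point just in front of the target, without sweeping.
; When close enough, it adds a fixed batch of its item class to the RobotCharacter's inventory and destroys itself.
; A missing item class prints an on-screen warning every tick.
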(event EventBeginPlay
  (|CallParentFunction) ; This node is disabled and will not be called.\nDrag off pins to build functionality.
)

(event Collision|EventActorBeginOverlap
  (params (OtherActor :type Actor%20Object%20Reference))
  (|CallParentFunction OtherActor) ; This node is disabled and will not be called.\nDrag off pins to build functionality.
)

(event EventTick
  (params (DeltaSeconds :type Float%20%28single-precision%29))
  (bind _self self)
  (bind _target (Variables|Default|GetTarget))
  (bind _target_2 (Variables|Default|GetTarget))
  (bind _returnvalue (Transformation|GetActorLocation _self))
  (if (Utilities|IsValidClass (Variables|Default|GetItemClass))
    (if (and (Variables|Default|GetisBeingSucked) (Utilities|IsValid (Variables|Default|GetTarget)))
      (Transformation|SetActorLocation (+ (* (* (Math|Vector|Normalize (- (+ (Transformation|GetActorLocation _target_2) (* (Transformation|GetActorForwardVector _target_2) 50)) _returnvalue)) DeltaSeconds) 1e+02) _returnvalue) false false)
      (if (<= (Math|Vector|Distance(Vector) (+ (Transformation|GetActorLocation _target) (* (Transformation|GetActorForwardVector _target) 25)) (Transformation|GetActorLocation self)) 1e+02)
        (bind _asrobot_character (Utilities|Casting|CastToRobotCharacter (Variables|Default|GetTarget)))
        (Default|AddItemtoInventory _asrobot_character (Variables|Default|GetItemClass) 12)
        (Variables|Default|SetisBeingSucked false)
        (Actor|DestroyActor)))
    (else
      (Development|PrintString "Set the item class!!!"))))

(fn ConstructionScript
  (|CallParentFunction))