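; Minigame task marker actor that shows a key-prompt text when the player is near an available task.
; Each Tick, it checks the GameMode's TasksMap for this task being incomplete and the preceding enum task complete, then tests player distance.
; Text alpha doubles as the visibility state, and toggling it sets or clears the player's CurrentMinigameTaskIndicator.
; ChangeMinigameState activates or deactivates the linked minigame camera.
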(event EventBeginPlay
  (bind _ascarbon_game_mode (Utilities|Casting|CastToCarbon_GameMode (Game|GetGameMode)))
  (Variables|Default|SetGameModeRef _ascarbon_game_mode))

(event EventTick
  (params (DeltaSeconds :type Float%20%28single-precision%29))
  (bind _gamemoderef (Variables|Default|GetGameModeRef))
  (bind _gamemoderef_2 (Variables|Default|GetGameModeRef))
  (bind _playerreference (Variables|/Game/MainGameAssets/Blueprints/GameMode/Carbon_GameMode.Carbon_GameMode_C|GetPlayerReference _gamemoderef_2))
  (bind _tasksmap (Variables|/Game/MainGameAssets/Blueprints/GameMode/Carbon_GameMode.Carbon_GameMode_C|GetTasksMap _gamemoderef))
  (if (and (== (.Value (Utilities|Map|Find _tasksmap (Variables|Default|GetTaskType))) false) (== (.Value (Utilities|Map|Find _tasksmap (Utilities|Enum|ByteToEnumTaskEnum (- (Variables|Default|GetTaskType) 1)))) true))
    (if (<= (Math|Vector|Distance(Vector) (Transformation|GetActorLocation) (Transformation|GetActorLocation (Variables|/Game/MainGameAssets/Blueprints/GameMode/Carbon_GameMode.Carbon_GameMode_C|GetPlayerReference (Variables|Default|GetGameModeRef)))) 2e+02)
      (if (== (.a (Variables|/Script/Engine.TextRenderComponent|GetTextRenderColor (Variables|/Script/Engine.TextRenderActor|GetTextRender (Variables|Default|GetEKeyIndicatorText)))) 0)
        (CallFunction|DisplayStartTaskIndicator true)
        (Variables|/Game/MainGameAssets/Blueprints/PlayerBlueprints/PlayerRobot_BP.PlayerRobot_BP_C|SetCurrentMinigameTaskIndicator _playerreference self))
      (elif (== (.a (Variables|/Script/Engine.TextRenderComponent|GetTextRenderColor (Variables|/Script/Engine.TextRenderActor|GetTextRender (Variables|Default|GetEKeyIndicatorText)))) 1)
        (CallFunction|DisplayStartTaskIndicator false)
        (Variables|/Game/MainGameAssets/Blueprints/PlayerBlueprints/PlayerRobot_BP.PlayerRobot_BP_C|SetCurrentMinigameTaskIndicator _playerreference 0)))))

(fn ConstructionScript)

(fn DisplayStartTaskIndicator
  (params (isShown :type Boolean))
  (bind _ekeyindicatortext (Variables|Default|GetEKeyIndicatorText))
  (bind _textrender (Variables|/Script/Engine.TextRenderActor|GetTextRender _ekeyindicatortext))
  (bind _textrendercolor (Variables|/Script/Engine.TextRenderComponent|GetTextRenderColor _textrender))
  (if isShown
    (Rendering|Components|TextRender|SetTextRenderColor _textrender (Math|Conversions|ToColor(LinearColor) (Math|Color|MakeColor (Math|Conversions|ToFloat(Byte) (.r _textrendercolor)) (Math|Conversions|ToFloat(Byte) (.g _textrendercolor)) (Math|Conversions|ToFloat(Byte) (.b _textrendercolor)))))
    (else
      (Rendering|Components|TextRender|SetTextRenderColor _textrender (Math|Conversions|ToColor(LinearColor) (Math|Color|MakeColor (Math|Conversions|ToFloat(Byte) (.r _textrendercolor)) (Math|Conversions|ToFloat(Byte) (.g _textrendercolor)) (Math|Conversions|ToFloat(Byte) (.b _textrendercolor)) 0.0))))))

(fn ChangeMinigameState
  (params (IsMinigameMode :type Boolean))
  (bind _minigamecam (Variables|Default|GetMinigameCam))
  (bind _cameracomponent (Variables|/Script/Engine.CameraActor|GetCameraComponent _minigamecam))
  (if IsMinigameMode
    (Components|Activation|Activate _cameracomponent false)
    (else
      (Components|Activation|Deactivate _cameracomponent))))