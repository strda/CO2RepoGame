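; AirFilterContainer slides an air filter part out for cleaning and retracts it once it is clean.
; While Activated, Tick steps the child actor along relative X by AscendDescend until it matches EndLocation.
; Otherwise Tick enables rotation on the AirFilterPart, then watches TotalDirt; at zero it reverses toward the origin and increments Carbon_GameMode's clean-filter count.
; Rotation is disabled once the part is back at the origin.
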(event EventBeginPlay)

(event Collision|EventActorBeginOverlap
  (params (OtherActor :type Actor%20Object%20Reference)))

(event EventTick
  (params (DeltaSeconds :type Float%20%28single-precision%29))
  (bind _childactor (Variables|Default|GetChildActor))
  (bind _relativelocation (Variables|/Script/Engine.SceneComponent|GetRelativeLocation _childactor))
  (bind _relativelocation_2 (Variables|/Script/Engine.SceneComponent|GetRelativeLocation _childactor))
  (if (and (Utilities|Operators|NotEqual(!=) _relativelocation (Variables|Default|GetEndLocation) 0.0) (Variables|Default|GetActivated))
    (Transformation|SetRelativeLocation _childactor (Math|Vector|MakeVector (+ (Variables|Default|GetAscendDescend) (.x _relativelocation_2)) (.y _relativelocation_2) (.z _relativelocation_2)) false false)
    (else
      (bind _asair_filter_part_blueprint (Utilities|Casting|CastToAirFilterPart_Blueprint (Variables|/Script/Engine.ChildActorComponent|GetChildActor (Variables|Default|GetChildActor))))
      (if (or (Variables|/Game/MainGameAssets/Blueprints/AirFilterPart_Blueprint.AirFilterPart_Blueprint_C|GetCanRotate _asair_filter_part_blueprint) (== (Variables|Default|GetAscendDescend) -1))
        (if (and (Utilities|Operators|EqualEqual _relativelocation (Variables|Default|GetEndLocation) 0.0) (== (Variables|Default|GetAscendDescend) -1))
          (Variables|/Game/MainGameAssets/Blueprints/AirFilterPart_Blueprint.AirFilterPart_Blueprint_C|SetCanRotate _asair_filter_part_blueprint false)
          (elif (<= (Variables|/Game/MainGameAssets/Blueprints/AirFilterPart_Blueprint.AirFilterPart_Blueprint_C|GetTotalDirt _asair_filter_part_blueprint) 0)
            (Variables|Default|SetAscendDescend -1)
            (Variables|Default|SetEndLocation "0, 0, 0")
            (bind _ascarbon_game_mode (Utilities|Casting|CastToCarbon_GameMode (Game|GetGameMode)))
            (Default|IncreaseFiltersClean _ascarbon_game_mode)))
        (else
          (Variables|/Game/MainGameAssets/Blueprints/AirFilterPart_Blueprint.AirFilterPart_Blueprint_C|SetCanRotate _asair_filter_part_blueprint true))))))

(fn ConstructionScript)