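; Navigation objective marker actor that marks a location and clears itself when reached.
; On any actor overlap while its mesh is visible, it hides and deactivates the mesh, then zeroes the render opacity of the directional arrow widget held by Carbon_GameMode.
; SetObjectiveVisibility is the shared toggle for showing or hiding the marker mesh, deactivating it only when hiding.
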(event Collision|EventActorBeginOverlap
  (params (OtherActor :type Actor%20Object%20Reference))
  (if (Rendering|IsVisible (Variables|Default|GetStaticMesh))
    (CallFunction|SetObjectiveVisibility false)
    (bind _ascarbon_game_mode (Utilities|Casting|CastToCarbon_GameMode (Game|GetGameMode)))
    (Widget|SetRenderOpacity (Variables|/Game/MainGameAssets/Blueprints/GameMode/Carbon_GameMode.Carbon_GameMode_C|GetDirectionalArrowRef _ascarbon_game_mode) 0.0)))

(fn ConstructionScript)

(fn SetObjectiveVisibility
  (params (IsVisible :type Boolean))
  (bind _staticmesh (Variables|Default|GetStaticMesh))
  (if IsVisible
    (Rendering|SetVisibility _staticmesh true false)
    (else
      (Rendering|SetVisibility _staticmesh false false)
      (Components|Activation|SetActive _staticmesh false false))))