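; DirtParticle is a dirt speck actor on an air filter that the player cleans by sweeping the cursor over it.
; It starts with a small random Health value, and each time the cursor enters its cube it loses one point.
; At zero it casts its parent actor to AirFilter_BP, decreases that filter's dirt total and destroys itself.
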(event OnBeginCursorOver(Cube)
  (params (TouchedComponent :type Primitive%20Component%20Object%20Reference))
  (bind _health (Variables|Default|GetHealth))
  (Math|Integer|DecrementInt _health
    (:%20%20
      (if (<= _health 0)
        (bind _asair_filter_bp (Utilities|Casting|CastToAirFilter_BP (Actor|GetParentActor)))
        (Default|DecreaseTotalDirt _asair_filter_bp)
        (Actor|DestroyActor)))))

(event EventBeginPlay
  (Variables|Default|SetHealth (Math|Random|RandomIntegerinRange 3 10)))

(event Collision|EventActorBeginOverlap
  (params (OtherActor :type Actor%20Object%20Reference)))

(event EventTick
  (params (DeltaSeconds :type Float%20%28single-precision%29)))

(fn ConstructionScript)