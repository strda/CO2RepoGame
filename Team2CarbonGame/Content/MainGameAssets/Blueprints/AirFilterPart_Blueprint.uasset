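; Air filter part that spawns random dirt particles on itself to be cleared, swapping the filter's material once none remain.
; BeginPlay and the duplicate Activation function copy the static mesh into a hidden procedural mesh, placing DirtParticle child actors on random vertices, re-rolled until within a local Y band.
; DecreaseTotalDirt counts down the remaining dirt.
; While CanRotate is set, Tick yaws the part using the RobotCharacter's axis input.
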(event EventBeginPlay
  (bind _output_get (Variables|Default|SetAmountOfDirt (Math|Random|RandomIntegerinRange 2 10)))
  (bind _output_get_2 (Variables|Default|SetTotalDirt _output_get))
  (Math|Integer|IncrementInt _output_get_2
    (:%20%20
      (Development|PrintString "Hello")
      (bind _returnvalue (AddComponent|AddProceduralMeshComponent false))
      (Class|KismetProceduralMeshLibrary|CopyProceduralMeshfromStaticMeshComponent (Variables|Debug|GetStaticMeshComponent) 0 _returnvalue false)
      (while (> (Variables|Default|GetAmountOfDirt) -1)
        (Math|Integer|DecrementInt (Variables|Default|GetAmountOfDirt)
          (:%20%20
            (bind _returnvalue_2 (AddComponent|AddChildActorComponent false))
            (ChildActorComponent|SetChildActorClass _returnvalue_2 "/Game/MainGameAssets/Blueprints/DirtParticle.DirtParticle_C")
            (Transformation|SetRelativeScale3D (Components|GetChildComponent _returnvalue_2 0) (Math|Conversions|ToVector(Float) (Math|Random|RandomFloatinRange 0.025 0.05)))
            (bind _vertices (Class|KismetProceduralMeshLibrary|GetSectionfromProceduralMesh _returnvalue (Math|Random|RandomIntegerinRange 0 (Class|ProceduralMeshComponent|GetNumSections _returnvalue)) :!label _label))
            (Transformation|SetRelativeLocation (Components|GetChildComponent _returnvalue_2 0) (Utilities|Array|Get(acopy) _vertices (Math|Random|RandomIntegerinRange 0 (Utilities|Array|Length _vertices))) false false)
            (while (or (> (.y (Variables|/Script/Engine.SceneComponent|GetRelativeLocation (Components|GetChildComponent _returnvalue_2 0))) -1e+01) (< (.y (Variables|/Script/Engine.SceneComponent|GetRelativeLocation (Components|GetChildComponent _returnvalue_2 0))) -31.0))
              (goto _label)))))
      (Rendering|SetVisibility _returnvalue false false))))

(event EventTick
  (params (DeltaSeconds :type Float%20%28single-precision%29))
  (bind _returnvalue (Transformation|GetActorRotation))
  (if (Variables|Default|GetCanRotate)
    (bind _asrobot_character (Utilities|Casting|CastToRobotCharacter (Game|Player|GetPlayerPawn 0)))
    (Transformation|SetActorRotation (Math|Rotator|MakeRotator (.roll _returnvalue) (.pitch _returnvalue) (+ (.yaw _returnvalue) (* (Variables|/Game/MainGameAssets/Blueprints/PlayerBlueprints/RobotCharacter.RobotCharacter_C|GetAxisValue _asrobot_character) 5.0))))))

(fn ConstructionScript)

(fn DecreaseTotalDirt
  (bind _result (Math|Integer|DecrementInt (Variables|Default|GetTotalDirt))
    (:%20%20
      (Development|PrintString (Utilities|String|ToString(Integer) _result))
      (if (<= _result 0)
        (Rendering|Material|SetMaterial (Variables|Default|GetAirFilter) 0 "/Game/MainGameAssets/Materials/lambert2.lambert2")))))

(fn Activation
  (bind _output_get (Variables|Default|SetAmountOfDirt (Math|Random|RandomIntegerinRange 2 10)))
  (bind _output_get_2 (Variables|Default|SetTotalDirt _output_get))
  (Math|Integer|IncrementInt _output_get_2
    (:%20%20
      (Development|PrintString "Hello")
      (bind _returnvalue (AddComponent|AddProceduralMeshComponent false))
      (Class|KismetProceduralMeshLibrary|CopyProceduralMeshfromStaticMeshComponent (Variables|Debug|GetStaticMeshComponent) 0 _returnvalue false)
      (while (> (Variables|Default|GetAmountOfDirt) -1)
        (Math|Integer|DecrementInt (Variables|Default|GetAmountOfDirt)
          (:%20%20
            (bind _returnvalue_2 (AddComponent|AddChildActorComponent false))
            (ChildActorComponent|SetChildActorClass _returnvalue_2 "/Game/MainGameAssets/Blueprints/DirtParticle.DirtParticle_C")
            (Transformation|SetRelativeScale3D (Components|GetChildComponent _returnvalue_2 0) (Math|Conversions|ToVector(Float) (Math|Random|RandomFloatinRange 0.025 0.05)))
            (bind _vertices (Class|KismetProceduralMeshLibrary|GetSectionfromProceduralMesh _returnvalue (Math|Random|RandomIntegerinRange 0 (Class|ProceduralMeshComponent|GetNumSections _returnvalue)) :!label _label))
            (Transformation|SetRelativeLocation (Components|GetChildComponent _returnvalue_2 0) (Utilities|Array|Get(acopy) _vertices (Math|Random|RandomIntegerinRange 0 (Utilities|Array|Length _vertices))) false false)
            (while (or (> (.y (Variables|/Script/Engine.SceneComponent|GetRelativeLocation (Components|GetChildComponent _returnvalue_2 0))) -1e+01) (< (.y (Variables|/Script/Engine.SceneComponent|GetRelativeLocation (Components|GetChildComponent _returnvalue_2 0))) -31.0))
              (goto _label)))))
      (Rendering|SetVisibility _returnvalue false false))))