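; TurnOffFactory is an interaction point, apparently for switching off a factory, that is revealed once the FactoryTask entry in the game mode's task map is true.
; Its box and indicator start hidden, and Tick polls Carbon_GameMode until that entry is true, then shows both once.
; Box overlaps set or clear the RobotCharacter's CurrentFacility regardless of that task state, as hiding only changes visibility.
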(event OnComponentBeginOverlap(Box)
  (params (OverlappedComponent :type Primitive%20Component%20Object%20Reference) (OtherActor :type Actor%20Object%20Reference) (OtherComp :type Primitive%20Component%20Object%20Reference) (OtherBodyIndex :type Integer) (bFromSweep :type Boolean) (SweepResult :type Hit%20Result%20Structure%20%28by%20ref%29))
  (bind _asrobot_character (Utilities|Casting|CastToRobotCharacter OtherActor))
  (Variables|/Game/MainGameAssets/Blueprints/PlayerBlueprints/RobotCharacter.RobotCharacter_C|SetCurrent%20Facility _asrobot_character self))

(event OnComponentEndOverlap(Box)
  (params (OverlappedComponent :type Primitive%20Component%20Object%20Reference) (OtherActor :type Actor%20Object%20Reference) (OtherComp :type Primitive%20Component%20Object%20Reference) (OtherBodyIndex :type Integer))
  (bind _asrobot_character (Utilities|Casting|CastToRobotCharacter OtherActor))
  (Variables|/Game/MainGameAssets/Blueprints/PlayerBlueprints/RobotCharacter.RobotCharacter_C|SetCurrent%20Facility _asrobot_character 0))

(event EventBeginPlay
  (Rendering|SetVisibility (Variables|Default|GetE_Indicator_BP) false false)
  (Rendering|SetVisibility (Variables|Default|GetBox) false false))

(event EventTick
  (params (DeltaSeconds :type Float%20%28single-precision%29))
  (if (not (Variables|Default|GetDone))
    (bind _ascarbon_game_mode (Utilities|Casting|CastToCarbon_GameMode (Game|GetGameMode)))
    (if (== (.Value (Utilities|Map|Find (Variables|/Game/MainGameAssets/Blueprints/GameMode/Carbon_GameMode.Carbon_GameMode_C|GetTasksMap _ascarbon_game_mode) (Variables|Default|GetFactoryTask))) true)
      (Rendering|SetVisibility (Variables|Default|GetBox) true false)
      (Rendering|SetVisibility (Variables|Default|GetE_Indicator_BP) true false)
      (Variables|Default|SetDone true))))

(fn ConstructionScript)