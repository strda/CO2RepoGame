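; Game mode for a robot environmental-cleanup game where carbon rises over time and reaching the maximum loses.
; Tick turns the carbon ratio into height fog opacity and sky Rayleigh tint as a visual warning.
; Check functions for trash, sorting, solar panels, air filters and tree planting feed CompleteTask, which updates the HUD, shows finish text and advances the task enum.
; Each completion lowers carbon, except the last enum task, which wins.
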(event EventBeginPlay
  (bind _returnvalue (Game|Player|GetPlayerPawn 0))
  ;[1 1 1] Initializing Game
  (bind _asrobot_character (Utilities|Casting|CastToRobotCharacter _returnvalue)
    (:then
      (Variables|Default|SetOtherPlayerRef _asrobot_character)
      (bind _returnvalue_2 (UserInterface|CreateWidget "/Game/MainGameAssets/UI/HUD_WBP.HUD_WBP_C" 0 self))
      (UserInterface|Viewport|AddtoViewport _returnvalue_2 0)
      (Variables|Default|SetHUDRef _returnvalue_2)
      (CallFunction|InitializeTasks))
    (:CastFailed
      (Utilities|Casting|CastToPlayerRobot_BP _returnvalue))))

(event EventTick
  (params (DeltaSeconds :type Float%20%28single-precision%29))
  (bind _initialskycolor (Variables|Default|GetInitialSkyColor))
  (bind _heightfog (Variables|Default|GetHeightFog))
  (Utilities|FlowControl|Sequence
    (:then_0
      (Variables|Default|SetCarbonLevel (+ (Variables|Default|GetCarbonLevel) DeltaSeconds))
      (if (>= (Variables|Default|GetCarbonLevel) (Variables|Default|GetMaxCarbonLevel))
        (CallFunction|LoseGame)))
    (:then_1
      (if (Utilities|IsValid _heightfog)
        (Class|ExponentialHeightFogComponent|SetFogMaxOpacity (Variables|/Script/Engine.ExponentialHeightFog|GetComponent _heightfog) (/ (Variables|Default|GetCarbonLevel) (Variables|Default|GetMaxCarbonLevel)))
        (Class|SkyAtmosphereComponent|SetRayleighScattering (Variables|/Script/Engine.SkyAtmosphere|GetSkyAtmosphereComponent (Variables|Default|GetSkyAtmosphere)) (Utilities|Struct|MakeLinearColor (Math|Float|Clamp(Float) (+ (/ (Variables|Default|GetCarbonLevel) (Variables|Default|GetMaxCarbonLevel)) (.r _initialskycolor))) (Math|Float|Clamp(Float) (+ (/ (Variables|Default|GetCarbonLevel) (Variables|Default|GetMaxCarbonLevel)) (.g _initialskycolor))) (.b _initialskycolor) 1.0))))))

(fn ConstructionScript)

(fn CompleteTask
  (params (TaskType :type TaskEnum%20Enum :default "NewEnumerator0"))
  (bind _returnvalue (+ TaskType 1))
  (bind _tasktextref (Variables|Default|GetTaskTextRef))
  (Utilities|Map|Add (Variables|Default|GetTasksMap) TaskType true)
  (Default|CheckTask (Variables|Default|GetHUDRef) TaskType)
  (bind (_textwidget _activetime) (Default|GetFinishTextfromTaskType _tasktextref TaskType))
  (Default|SetTextVisible _tasktextref _textwidget)
  (Default|DisableText _tasktextref _activetime _textwidget)
  (if (< _returnvalue (|GetNumEnumEntries))
    (Variables|Default|SetCurrentTask (Utilities|Enum|ByteToEnumTaskEnum _returnvalue))
    (Variables|Default|SetCarbonLevel (Math|Float|Clamp(Float) (- (Variables|Default|GetCarbonLevel) 3e+01) 0.0 (Variables|Default|GetMaxCarbonLevel)))
    (else
      (CallFunction|WinGame))))

(fn InitializeTasks
  (bind _enumvalue (|ForEachTaskEnum)
    (:LoopBody
      (Utilities|Map|Add (Variables|Default|GetTasksMap) _enumvalue false))))

(fn CheckGarbageCollectionTask
  (if (== (.Value (Utilities|Map|Find (Variables|/Game/MainGameAssets/Blueprints/PlayerBlueprints/RobotCharacter.RobotCharacter_C|GetInventory (Variables|Default|GetOtherPlayerRef)) "/Game/MainGameAssets/Items/Trash.Trash_C")) 15)
    (CallFunction|CompleteTask "NewEnumerator0")))

(fn CompleteAirFilter
  (bind _result (Math|Integer|IncrementInt (Variables|Default|GetFiltersComplete))
    (:%20%20
      (if (>= _result 4)
        (CallFunction|CompleteTask "NewEnumerator3")))))

(fn CheckSortingCompletion
  (if (>= (Variables|Default|GetrecyclablesSorted) 15)
    (CallFunction|CompleteTask "NewEnumerator1")))

(fn WinGame
  (bind _returnvalue (UserInterface|CreateWidget "/Game/MainGameAssets/UI/WinScreen_WBP.WinScreen_WBP_C"))
  (UserInterface|Viewport|AddtoViewport _returnvalue 0)
  (Game|SetGamePaused true))

(fn LoseGame
  (bind _returnvalue (UserInterface|CreateWidget "/Game/MainGameAssets/UI/LoseScreen_WBP.LoseScreen_WBP_C"))
  (UserInterface|Viewport|AddtoViewport _returnvalue 0)
  (Game|SetGamePaused true))

(fn InitilizeSolarPanel
  (Rendering|SetActorHiddenInGame (Variables|SolarPanelGame|GetSolarPanelOne) false)
  (Rendering|SetActorHiddenInGame (Variables|SolarPanelGame|GetSolarPanelTwo) false)
  (Rendering|SetActorHiddenInGame (Variables|solarPanelGame|GetSolarPanelThree) false)
  (bind _assolar_panel_part_despensor (Utilities|Casting|CastTosolarPanelPartDespensor (Variables|SolarPanelGame|GetSolarPartSpawner)))
  (Default|SpawnParts _assolar_panel_part_despensor))

(fn IsSolarPanelFinished
  (Math|Integer|CompareInt (Variables|SolarPanelGame|GetSolarPanelsFinished) 3
    (:==
      (CallFunction|CompleteTask "NewEnumerator2"))))

(fn SetNextObjectiveLocation
  (bind _objectivelocations (Variables|Default|GetObjectiveLocations))
  (Default|SetObjectiveVisibility (Variables|Default|GetCurrentObjectiveLocation) false)
  (bind _output_get (Variables|Default|SetCurrentObjectiveLocation (Utilities|Array|Get(acopy) _objectivelocations (+ (Utilities|Array|FindItem _objectivelocations (Variables|Default|GetCurrentObjectiveLocation)) 1))))
  (Default|SetObjectiveVisibility _output_get true)
  (Widget|SetRenderOpacity (Variables|Default|GetDirectionalArrowRef) 1.0))

(fn StumpRemovalCheck
  (Math|Integer|CompareInt (Variables|TreeMiniGame|GetStumpsCollected) 12
    (:>
      _)
    (:==
      _))
  (Variables|TreeMiniGame|SetallStumpsCollected true))

(fn MakeMoundsVisible
  (if (not (Variables|TreeMiniGame|GetMoundAreVisible))
    (for _array_element (Variables|TreeMiniGame|GetallMounds)
      (Rendering|SetVisibility (Variables|/Game/MainGameAssets/Items/TreeMinigame_objects/DirtMound.DirtMound_C|GetmoundBody _array_element) true false))
    (Variables|TreeMiniGame|SetMoundAreVisible true)))

(fn TreeTaskCheck
  (CallFunction|StumpRemovalCheck)
  (if (Variables|TreeMiniGame|GetallStumpsCollected)
    (CallFunction|MakeMoundsVisible)
    (Math|Integer|CompareInt (Variables|TreeMiniGame|GetTreesPlanted) 12
      (:==
        (CallFunction|CompleteTask "NewEnumerator0")))))