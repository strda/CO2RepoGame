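; TaskLockedDoor is a door that stays shut until a required task is marked complete.
; Each Tick, it polls the TasksMap in Carbon_GameMode for its TaskNeeded entry.
; Once that entry is true, it snaps the static mesh to a fixed open rotation and sets a Completed flag that skips further checks.
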(event EventBeginPlay)

(event Collision|EventActorBeginOverlap
  (params (OtherActor :type Actor%20Object%20Reference)))

(event EventTick
  (params (DeltaSeconds :type Float%20%28single-precision%29))
  (if (not (Variables|Default|GetCompleted))
    (bind _ascarbon_game_mode (Utilities|Casting|CastToCarbon_GameMode (Game|GetGameMode)))
    (if (== (.Value (Utilities|Map|Find (Variables|/Game/MainGameAssets/Blueprints/GameMode/Carbon_GameMode.Carbon_GameMode_C|GetTasksMap _ascarbon_game_mode) (Variables|Default|GetTaskNeeded))) true)
      (Transformation|SetRelativeRotation (Variables|Default|GetStaticMesh) "0.000000,120.000000,0.000000" false false)
      (Variables|Default|SetCompleted true))))

(fn ConstructionScript)